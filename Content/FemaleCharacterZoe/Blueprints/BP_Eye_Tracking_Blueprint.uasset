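; Moving look-at target actor that drives eye tracking on a referenced character.
; It stores its starting location on BeginPlay, then each Tick teleports along an elliptical sine/cosine path in the YZ plane, driven by game time.
; The same computed position is written to the character's EyeLookAt every frame, so that value follows the moving actor.
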(event EventBeginPlay
  (Variables|Default|SetInitial%20Location (Transformation|GetActorLocation)))

(event EventTick
  (params (DeltaSeconds :type Float%20%28single-precision%29))
  (bind _returnvalue (Utilities|Time|GetGameTimeinSeconds))
  (bind _initial_location (Variables|Default|GetInitial%20Location))
  (bind _returnvalue_2 (Math|Trig|Sin(Radians) _returnvalue))
  (bind _returnvalue_3 (Math|Trig|Cos(Radians) _returnvalue))
  (bind _returnvalue_4 (* _returnvalue_3 1e+01))
  (bind _returnvalue_5 (* _returnvalue_2 3e+01))
  (bind _returnvalue_6 (Math|Vector|MakeVector 0.0 _returnvalue_5 _returnvalue_4))
  (bind _returnvalue_7 (+ _initial_location _returnvalue_6))
  (Transformation|SetActorLocation _returnvalue_7 false true)
  (Variables|/Game/FemaleCharacterZoe/Blueprints/BP_FemaleCharacterZoe.BP_FemaleCharacterZoe_C|SetEye%20Look%20At (Variables|Default|GetCharacter) _returnvalue_7))

(fn ConstructionScript)